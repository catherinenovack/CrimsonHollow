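; Base pickup Blueprint that the third-person player can interact with, with empty VariaçõesDeComportamento and Body events as apparent hooks for child variants.
; Sphere overlap registers the pickup as the player's last interactable and look-at target and sets CanInteract.
; Leaving the sphere clears CanInteract and the look-at flag.
; Interact runs the behaviour hook, destroys the actor and prints an added-to-inventory message, with no inventory logic here.
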(event OnComponentBeginOverlap(Sphere)
  (params (OverlappedComponent :type Primitive%20Component%20Object%20Reference) (OtherActor :type Actor%20Object%20Reference) (OtherComp :type Primitive%20Component%20Object%20Reference) (OtherBodyIndex :type Integer) (bFromSweep :type Boolean) (SweepResult :type Hit%20Result%20Structure%20%28by%20ref%29))
  (bind _asbp_third_person_character_player (Utilities|Casting|CastToBP_ThirdPersonCharacter_Player OtherActor))
  (Variables|/Game/BP/CoreGameplay/BP_ThirdPersonCharacter_Player.BP_ThirdPersonCharacter_Player_C|SetLastInteractObj _asbp_third_person_character_player self)
  (Variables|Default|SetCanInteract? true)
  ;[0.15 0.15 0.15 0.5] Look at
  (Variables|/Game/BP/CoreGameplay/BP_ThirdPersonCharacter_Player.BP_ThirdPersonCharacter_Player_C|SetIsLookAt_0 _asbp_third_person_character_player true)
  (Variables|/Game/BP/CoreGameplay/BP_ThirdPersonCharacter_Player.BP_ThirdPersonCharacter_Player_C|SetLookAtActor _asbp_third_person_character_player self))

(event OnComponentEndOverlap(Sphere)
  (params (OverlappedComponent :type Primitive%20Component%20Object%20Reference) (OtherActor :type Actor%20Object%20Reference) (OtherComp :type Primitive%20Component%20Object%20Reference) (OtherBodyIndex :type Integer))
  (bind _asbp_third_person_character_player (Utilities|Casting|CastToBP_ThirdPersonCharacter_Player OtherActor))
  (Variables|Default|SetCanInteract? false)
  ;[0.15 0.15 0.15 0.5] Look at
  (Variables|/Game/BP/CoreGameplay/BP_ThirdPersonCharacter_Player.BP_ThirdPersonCharacter_Player_C|SetIsLookAt_0 _asbp_third_person_character_player false))

(event Custom|Body)

(event Custom|Variações%20de%20comportamento)

(event EventInteract
  (CallFunction|VariaçõesDeComportamento)
  (Actor|DestroyActor)
  (Development|PrintString "Adicionado ao inventário"))

(fn ConstructionScript)